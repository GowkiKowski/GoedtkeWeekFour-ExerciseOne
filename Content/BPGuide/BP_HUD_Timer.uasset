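; BP_HUD_Timer is a HUD Blueprint that shows an elapsed-time counter on screen.
; On BeginPlay it starts a looping one-second timer whose event increments a Time counter.
; DrawHUD draws that value each frame as scaled green "Time:" text near the top-left corner, using canvas DrawText rather than a widget.
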(event `self.ReceiveBeginPlay`
  (`KismetSystemLibrary.K2_SetTimerDelegate` (delegate `Count`) 1.0 true))

(event `Count`
  (set `self.Time` (+ (`self.Time`) 1)))

(event `self.ReceiveDrawHUD`
  (params (SizeX :type Integer) (SizeY :type Integer))
  (`self.DrawText` (`KismetTextLibrary.Conv_TextToString` (`KismetTextLibrary.Conv_StringToText` (`KismetStringLibrary.BuildString_Int` "Time:" "" (`self.Time`)))) (struct :`G` 0.473958 :`B` 0.031341 :`A` 1.0) 20.0 10.0 null 5.0))

(fn `UserConstructionScript`)